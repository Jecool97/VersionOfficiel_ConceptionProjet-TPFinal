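; BP_RouteInfini is an endless-road segment that scrolls along Y past the VR player's car.
; BeginPlay plays engine sound at the car and stores building and vehicle lists, unused here.
; Box overlap asks VRGameMode for a new route, then destroys this segment after a delay; GetNextSpawn returns the Arrow's transform.
; Every tick, each segment moves all segments at a base or accelerated speed, without delta-time scaling.
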(event `self.ReceiveBeginPlay`
  ;[1 1 1] Déclare le joueur pour ses variables et Events et stock les différents mesh de maison/Voiture dans des arrays afin de les générés aléatoirement lors de l'apparition d'une nouvelle route
  (bind _asvrpawn (cast `/Game/Blueprint/VRPawn` (`GameplayStatics.GetPlayerPawn` 0)))
  (bind _output_get (set `self.As VRPawn` _asvrpawn))
  (`GameplayStatics.PlaySoundAtLocation` (`self.SonMoteur`) (`SceneComponent.K2_GetComponentLocation` (`/Game/Blueprint/VRPawn.Voiture` _output_get)) (struct) 1.0 1.0 0.0 null null null null)
  (set `self.LotsVoiture` (`|MakeArray` (`self.Voiture06`) (`self.Voiture05`) (`self.Voiture04`) (`self.Voiture03`) (`self.Voiture02`) (`self.Voiture01`)))
  (set `self.LotsImmeuble` (`|MakeArray` (`self.Immeuble02`) (`self.Immeuble01`))))

(event `self.Box.OnComponentBeginOverlap`
  (params (OverlappedComponent :type "PrimitiveComponent Object Reference") (OtherActor :type "Actor Object Reference") (OtherComp :type "PrimitiveComponent Object Reference") (OtherBodyIndex :type Integer) (bFromSweep :type Boolean) (SweepResult :type "HitResult Structure (by ref)"))
  ;[1 1 1] Ajout de nouvelle route lorsque le joueur passe dans la zone de collision d'une route  et détruit ceux qui se trouve à l'arrière du joueur après un certain délai
  (bind _asvrgame_mode (cast `/Game/VRTemplate/Blueprints/VRGameMode` (`GameplayStatics.GetGameMode`)))
  (`/Game/VRTemplate/Blueprints/VRGameMode.AddNewRoute` _asvrgame_mode)
  (`KismetSystemLibrary.Delay` 4.0)
  (`self.K2_DestroyActor`))

(event `Acceleration`
  (params (VitesseDeplacement :type "Float (double-precision)") (Acceleration :type Boolean))
  ;[1 1 1] Donne une vitesse contante raisonnable en continue à la route pou accélère si le joueur appuie la touche d'accélération
  (if Acceleration :!label _label
    (set `self.VitesseDeplacement` VitesseDeplacement)
    (else
      (set `self.VitesseDeplacement` 5.0)))
  (bind _outactors (`GameplayStatics.GetAllActorsOfClass` "BP_RouteInfini_C"))
  (for _array_element _outactors
    (`self.K2_AddActorWorldTransform` _array_element (`KismetMathLibrary.MakeTransform` (`KismetMathLibrary.MakeVector` 0.0 (`self.VitesseDeplacement`))) false false)))

(event `self.ReceiveTick`
  (params (DeltaSeconds :type "Float (single-precision)"))
  ;[1 1 1] Donne une vitesse contante raisonnable en continue à la route pou accélère si le joueur appuie la touche d'accélération
  (goto _label))

(fn `GetNextSpawn`
  (returns (ReturnValue :type "Transform Structure"))
  (bind (_returnvalue_location _returnvalue_rotation) (`KismetMathLibrary.BreakTransform` (`SceneComponent.K2_GetComponentToWorld` (`self.Arrow`))))
  (return (`KismetMathLibrary.MakeTransform` _returnvalue_location _returnvalue_rotation)))

(fn `UserConstructionScript`)