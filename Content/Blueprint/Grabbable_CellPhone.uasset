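; A grabbable cell phone actor that returns to its spawn point when it is not held in the hand.
; On BeginPlay and whenever the static mesh registers a hit while not held, ResetPosition teleports the mesh to the SpawnTelephone transform.
; MessageUrgent flags a message as received, and as answered if the phone is held and sending is enabled.
; A second response event is empty, and the phone UI widget creation is left unconnected.
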(event `self.ReceiveBeginPlay`
  (`self.ResetPosition` (stale `ResetPosition` `Spawn Telephone`)))

(event `ResetPosition`
  (params (`Spawn Telephone` :type "Transform Structure") (TelephoneENMain :type Boolean))
  (if (not TelephoneENMain)
    (`SceneComponent.K2_SetWorldTransform` (`self.StaticMesh`) `Spawn Telephone` false true)))

(event `self.StaticMesh.OnComponentHit`
  (params (HitComponent :type "PrimitiveComponent Object Reference") (OtherActor :type "Actor Object Reference") (OtherComp :type "PrimitiveComponent Object Reference") (NormalImpulse :type "Vector Structure") (Hit :type "HitResult Structure (by ref)"))
  (if (not (`self.TelephoneEnMain?`))
    (`self.ResetPosition` (stale `ResetPosition` `Spawn Telephone`))))

(event `MessageUrgent`
  (set `self.MessageRecu?` true)
  (if (and (`self.TelephoneEnMain?`) (`self.EnvoieMessage?`))
    (set `self.MessageRepondu?` true)))

(event `ReponseDeuxMessage`)

(fn `UserConstructionScript`)